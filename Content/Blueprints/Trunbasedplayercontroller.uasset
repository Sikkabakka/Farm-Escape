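; Player controller for a turn-based grid game that handles mouse selection and movement of BP_Hero units.
; Left click traces under the cursor to select a hero and cache its tile, with a branch calling the move event when no new actor is valid.
; That event runs BP_grid's A* pathfinding to the cursor tile, creates path instances and teleports the hero to the path's first element.
; A step-by-step MoveA* helper exists but is never called here.
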(event EventBeginPlay
  (bind _outactors (Actor|GetAllActorsOfClass "/Game/Grid/BP_grid.BP_grid_C"))
  (Variables|Default|SetBP_Grid (Utilities|Array|Get(acopy) _outactors))
  (Variables|Default|SetBP_Pathfinding (Variables|/Game/Grid/BP_grid.BP_grid_C|GetPathfinding (Utilities|Array|Get(acopy) _outactors))))

(event EventTick
  (params (DeltaSeconds :type Float%20%28single-precision%29)))

(event Custom|Server%20Action%20-%20Move%20Hero
  (params (Hero :type BP%20Hero%20Object%20Reference) (Location :type Vector))
  (bind _bp_pathfinding (Variables|Default|GetBP_Pathfinding))
  (bind _index (Default|GetTileIndexUnderCursor (Variables|Default|GetBP_Grid)))
  (bind _path (Default|DoA* _bp_pathfinding (Variables|Default|GetActorIndex) _index))
  (Default|MakeInstances _bp_pathfinding _path)
  (for _array_element _path
    (bind _worldlocation (Default|GetWorldLocationfromIndex (Variables|Default|GetBP_Grid) (Utilities|Array|Get(acopy) _path)))
    (Transformation|SetWorldLocation (Variables|/Script/Engine.Character|GetCapsuleComponent (Variables|Default|GetSelectedHero)) _worldlocation false false)
    (Development|PrintString (Utilities|String|ToString(Vector) _worldlocation)))
  (Transformation|SetWorldLocation (Variables|/Script/Engine.Character|GetCapsuleComponent (Variables|Default|GetSelectedHero)) _worldlocation false false))

(event Input|MouseEvents|LeftMouseButton
  (params (Key :type Key%20Structure :default "None"))
  (:Pressed
    (CallFunction|HandleLeftMouseButton)))

(fn ConstructionScript)

(fn HandleLeftMouseButton
  (bind _returnvalue (Game|GetPlayerController 0))
  (bind (_worldlocation _worlddirection) (Game|Player|ConvertMouseLocationToWorldSpace _returnvalue))
  (Utilities|FlowControl|Sequence
    (:then_0
      (bind _outhit (Collision|LineTraceByChannel _worldlocation (+ _worldlocation (* _worlddirection 5e+03)) "TraceTypeQuery2" false 0 "None" false))
      (bind _output_get (LocalVariables|Setnewlyselectedlocation (.Location (Collision|BreakHitResult _outhit))))
      (Development|PrintString (Utilities|String|ToString(Vector) _output_get))
      (Development|PrintString (Utilities|GetDisplayName (.HitActor (Collision|BreakHitResult _outhit))))
      (bind _asbp_hero (Utilities|Casting|CastToBP_Hero (.HitActor (Collision|BreakHitResult _outhit)))
        (:then
          (LocalVariables|SetNewlySelectedActor _asbp_hero))
        (:CastFailed
          (Development|PrintString "not player"))))
    (:then_1
      (if (!= (Variables|Default|GetSelectedHero) (LocalVariables|GetNewlySelectedActor))
        (LocalVariables|GetNewlySelectedActor
          (:then
            (Development|PrintString "ny")
            (bind _output_get_2 (Variables|Default|SetSelectedHero (LocalVariables|GetNewlySelectedActor)))
            (bind _index (Default|GetTileIndexfromWorldLocation (Variables|Default|GetBP_Grid) (Transformation|GetWorldLocation (Variables|/Script/Engine.Actor|GetRootComponent _output_get_2))))
            (Variables|Default|SetActorIndex _index))
          (:else
            (bind _selectedhero (Variables|Default|GetSelectedHero)
              (:then
                (CallFunction|ServerAction-MoveHero _selectedhero (LocalVariables|Getnewlyselectedlocation))
                (Variables|Default|SetSelectedHero 0))
              (:else))))
        (else
          (Development|PrintString "Samme"))))))

(fn MoveA*
  (params (Path :type Array%20of%20Int%20Point%20Structures) (Target :type BP%20Hero%20Object%20Reference))
  (bind _output_get (LocalVariables|SetPATHEN Path))
  (LocalVariables|SetTARGETEN Target)
  (Utilities|Array|Reverse _output_get)
  (bind _worldlocation (Default|GetWorldLocationfromIndex (Variables|Default|GetBP_Grid) (Utilities|Array|Get(acopy) (LocalVariables|GetPATHEN) (Variables|Default|GetIncrementInt))))
  (Transformation|SetWorldLocation (Variables|/Script/Engine.Actor|GetRootComponent (LocalVariables|GetTARGETEN)) _worldlocation false false)
  (Variables|Default|SetIncrementInt (+ (Variables|Default|GetIncrementInt) 1))
  (return 0))