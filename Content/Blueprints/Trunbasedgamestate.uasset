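; Turn-based game state that tracks which of two turns is active.
; On BeginPlay it shows the mouse cursor, resets the turn through StartGame, then creates the UI widget and adds it to the viewport.
; The ChangeTurn event uses the CheckTurn function to flip the Turn value between 0 and 1.
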(event Custom|StartGame
  (Variables|Default|SetTurn 0))

(event Custom|ChangeTurn
  (bind _turn (CallFunction|CheckTurn))
  (if _turn
    (Variables|Default|SetTurn 1)
    (else
      (Variables|Default|SetTurn 0))))

(event EventBeginPlay
  (Variables|/Script/Engine.PlayerController|SetbShowMouseCursor (Game|GetPlayerController 0) true)
  (CallFunction|StartGame)
  (bind _returnvalue (UserInterface|CreateWidget "/Game/Blueprints/UI.UI_C"))
  (UserInterface|Viewport|AddtoViewport _returnvalue 0))

(fn ConstructionScript)

(fn CheckTurn
  (if (== 0 (Variables|Default|GetTurn))
    (return true)
    (else
      (return false))))