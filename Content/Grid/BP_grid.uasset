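; Isometric grid actor that builds a tile field and maps the mouse cursor to tile indices, printing the index every tick.
; The construction script clears and refills an instanced static mesh with tiles in a staggered diamond layout.
; Cursor location comes from a channel trace (hit Y/Z remapped to X/Y), falling back to line-plane intersection.
; Indices come from inverting two basis vectors after subtracting an offset; AddStateToTile is an empty stub.
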(event EventBeginPlay)

(event Collision|EventActorBeginOverlap
  (params (OtherActor :type Actor%20Object%20Reference)))

(event EventTick
  (params (DeltaSeconds :type Float%20%28single-precision%29))
  (bind _location (CallFunction|GetCursorLocationonGrid))
  (bind (_index _returnvalue _returnvalue1 _output_get _output_get1) (CallFunction|GetTileIndexfromWorldLocation _location))
  (Development|PrintString (Utilities|String|ToString(Integer) _index)))

(fn ConstructionScript
  (CallFunction|SpawnGrid (Variables|Default|GetGridStartLocation) (Variables|Default|GetGridTileSize) (Variables|Default|GetGridTileCount)))

(fn SpawnGrid
  (params (StartLocation :type Vector) (TileSize :type Vector) (TileCount :type Vector%202D%20Structure))
  (Variables|Default|SetGridStartLocation StartLocation)
  (Variables|Default|SetGridTileSize TileSize)
  (Variables|Default|SetGridTileCount TileCount)
  (CallFunction|NewFunction0)
  (Components|StaticMesh|SetStaticMesh (Variables|Default|GetInstancedStaticMesh) "/Game/Grid/GridShapes/IsometricCube/IsometricTilerBottom.IsometricTilerBottom")
  (for _index (range 0 (- (Math|Float|Round (.x (Variables|Default|GetGridTileCount))) 1))
    (LocalVariables|Setx _index)
    (for _index_2 (range 0 (- (Math|Float|Round (.y (Variables|Default|GetGridTileCount))) 1))
      (LocalVariables|Sety _index_2)
      (LocalVariables|SetTileTransform (Math|Transform|MakeTransform (+ (Variables|Default|GetGridStartLocation) (Math|Vector|MakeVector (+ (* (Math|Conversions|ToFloat(Integer) (LocalVariables|Getx)) 32.0) (* (Math|Conversions|ToFloat(Integer) (LocalVariables|Gety)) 32.0)) (+ (* (Math|Conversions|ToFloat(Integer) (LocalVariables|Getx)) 64.0) (* (Math|Conversions|ToFloat(Integer) (LocalVariables|Gety)) -64.0)) 0.0)) "0,90.000000,0.000000" "1.000000,1.000000,1.000000"))
      (Components|InstancedStaticMesh|AddInstance (Variables|Default|GetInstancedStaticMesh) (LocalVariables|GetTileTransform) false))))

(fn NewFunction0
  (Components|InstancedStaticMesh|ClearInstances (Variables|Default|GetInstancedStaticMesh)))

(fn GetCursorLocationonGrid
  (params (PlayerIndex :type Integer))
  (bind _returnvalue (Game|GetPlayerController PlayerIndex))
  (bind _gridstartlocation (Variables|Default|GetGridStartLocation))
  (bind (_hitresult _returnvalue_2) (Game|Player|GetHitResultUnderCursorbyChannel _returnvalue "TraceTypeQuery3" false))
  (bind (_worldlocation _worlddirection) (Game|Player|ConvertMouseLocationToWorldSpace _returnvalue))
  (bind _returnvalue_3 (Class|KismetMathLibrary|MakePlanefromPointandNormal _gridstartlocation "0, 0, 0"))
  (bind _location (Collision|BreakHitResult _hitresult))
  (bind _returnvalue_4 (* _worlddirection "9999.000000,9999.000000,9999.000000"))
  (bind _returnvalue_5 (+ _worldlocation _returnvalue_4))
  (bind (_t _intersection _returnvalue_6) (Class|KismetMathLibrary|LinePlaneIntersection _worldlocation _returnvalue_5 _returnvalue_3))
  (if _returnvalue_2
    (return (Math|Vector|MakeVector (.y _location) (.z _location) 0.0))
    (elif _returnvalue_6
      (return _intersection)
      (else
        (return "-999.000000,-999.000000,-999.000000")))))

(fn GetTileIndexfromWorldLocation
  (params (Location :type Vector))
  (bind _enhetsvektory (LocalVariables|GetEnhetsvektorY))
  (bind _enhetsvektorx (LocalVariables|GetEnhetsVektorx))
  (bind _enhetsvektory_2 (LocalVariables|GetEnhetsvektorY))
  (bind _enhetsvektorx_2 (LocalVariables|GetEnhetsVektorx))
  (bind _enhetsvektory_3 (LocalVariables|GetEnhetsvektorY))
  (bind _offsett (LocalVariables|GetOffsett))
  (bind _returnvalue (- Location _offsett))
  (Development|PrintString (Utilities|String|ToString(Vector) _returnvalue))
  (LocalVariables|Setlocation%20on%20grid _returnvalue)
  (if true
    (bind _output_get (LocalVariables|SetY (/ (- (* (.y (LocalVariables|Getlocation%20on%20grid)) (.x (LocalVariables|GetEnhetsVektorx))) (* (.y (LocalVariables|GetEnhetsVektorx)) (.x (LocalVariables|Getlocation%20on%20grid)))) (- (* (.x _enhetsvektorx) (.y _enhetsvektory_2)) (* (.y _enhetsvektorx) (.x _enhetsvektory_2))))))
    (bind _output_get_2 (LocalVariables|SetX (/ (+ (* (.y (LocalVariables|Getlocation%20on%20grid)) (* (.x _enhetsvektory) -1.0)) (* (.y _enhetsvektory) (.x (LocalVariables|Getlocation%20on%20grid)))) (- (* (.x _enhetsvektorx_2) (.y _enhetsvektory_3)) (* (.y _enhetsvektorx_2) (.x _enhetsvektory_3))))))
    (return (Utilities|Struct|MakeIntPoint (Math|Float|Truncate _output_get_2) (Math|Float|Truncate _output_get)) "" "" _output_get_2 _output_get)
    (else
      (return (Utilities|Struct|MakeIntPoint -999 -999) "" "" 0.0 0.0))))

(fn GetTileIndexUnderCursor
  (params (PlayerIndex :type Integer))
  (bind _location (CallFunction|GetCursorLocationonGrid PlayerIndex))
  (bind (_index _returnvalue _returnvalue1) (CallFunction|GetTileIndexfromWorldLocation _location))
  (return _index _returnvalue _returnvalue1))

(fn AddStatetoTile
  (params (index :type Int%20Point%20Structure) (NewParam1 :type E_Tilestate%20Enum :default "NewEnumerator0")))