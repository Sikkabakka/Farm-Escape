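; BP_grid_2 is an unfinished grid actor, apparently meant to build a tile grid from an instanced static mesh.
; Its construction script passes the start location, tile size and tile count variables into SpawnGrid, which stores them and assigns the IsometricTilerBottom mesh.
; The loop over the X tile count has an empty body and a disconnected index assignment, so no instances are added.
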(event EventBeginPlay)

(event Collision|EventActorBeginOverlap
  (params (OtherActor :type Actor%20Object%20Reference)))

(event EventTick
  (params (DeltaSeconds :type Float%20%28single-precision%29)))

(fn ConstructionScript
  (CallFunction|SpawnGrid (Variables|Default|GetGridStartLocation) (Variables|Default|GetGridTileSize) (Variables|Default|GetGridTileCount)))

(fn SpawnGrid
  (params (StartLocation :type Vector) (TileSize :type Vector) (TileCount :type Vector%202D%20Structure))
  (Variables|Default|SetGridStartLocation StartLocation)
  (Variables|Default|SetGridTileSize TileSize)
  (Variables|Default|SetGridTileCount TileCount)
  (Components|StaticMesh|SetStaticMesh (Variables|Default|GetInstancedStaticMesh) "/Game/Grid/GridShapes/IsometricCube/IsometricTilerBottom.IsometricTilerBottom")
  (for _index (range 0 (- (Math|Float|Round (.x (Variables|Default|GetGridTileCount))) 1))
    _))